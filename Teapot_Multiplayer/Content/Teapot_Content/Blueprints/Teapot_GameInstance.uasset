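; Game instance for the Teapot game that handles hosting and joining multiplayer sessions.
; Hosting is allowed only from the initial state; it creates a LAN session, opens the first scenario level as a listen server, then advances CurrentState.
; Joining connects to a supplied search result without checking or changing the state, which GetCurrentState exposes.
; Session outcomes and refused host attempts are reported only through debug prints.
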(event Custom|HostGameEvent
  ;[1 1 1] Host game session
  (if (Utilities|Enum|Equal(Enum) (Variables|Default|GetCurrentState) "NewEnumerator0")
    (|Session (Game|GetPlayerController 0) 4 true
      (:OnSuccess
        (Development|PrintString "Succeded creating session")
        (Game|OpenLevel(byName) "Teapot_Level_Scenario_0" true "listen")
        (Variables|Default|SetCurrentState "NewEnumerator1"))
      (:OnFailure
        (Development|PrintString "Error creating session")))
    (else
      (Development|PrintString "Can't host game while already in session"))))

(event Custom|JoinGameEvent
  (params (SessionToJoin :type Blueprint%20Session%20Result%20Structure))
  ;[1 1 1] Join game session
  (|JoinSession (Game|GetPlayerController 0) SessionToJoin
    (:OnSuccess
      (Development|PrintString "Successfully Joined session"))
    (:OnFailure
      (Development|PrintString "Error connecting to session"))))

(fn GetCurrentState
  (return (Variables|Default|GetCurrentState)))