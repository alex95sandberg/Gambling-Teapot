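; Victory trigger box that ends the game when a Teapot_Victory_Weapon held by a motion controller overlaps it.
; The overlap clears the controller's attached actor, destroys the weapon and reveals a static battery in its place.
; A delayed sequence then toggles two spotlights, fades every player's camera and audio to black, and adds the victory widget for each player controller.
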(event OnComponentBeginOverlap(Box)
  (params (OverlappedComponent :type Primitive%20Component%20Object%20Reference) (OtherActor :type Actor%20Object%20Reference) (OtherComp :type Primitive%20Component%20Object%20Reference) (OtherBodyIndex :type Integer) (bFromSweep :type Boolean) (SweepResult :type Hit%20Result%20Structure%20%28by%20ref%29))
  (bind _asteapot_victory_weapon (Utilities|Casting|CastToTeapot_Victory_Weapon OtherActor))
  (bind _asteapot_motion_controller (Utilities|Casting|CastToTeapot_MotionController (Actor|GetAttachParentActor _asteapot_victory_weapon)))
  (Variables|/Game/Teapot_Content/Blueprints/Teapot_MotionController.Teapot_MotionController_C|SetAttachedActor _asteapot_motion_controller 0)
  (Actor|DestroyActor _asteapot_victory_weapon)
  (Rendering|SetVisibility (Variables|Default|GetStaticBattery) true false)
  (Utilities|FlowControl|Delay 0.5)
  (Rendering|SetVisibility (Variables|Default|GetSpotLight1) true true)
  (Utilities|FlowControl|Delay 0.3)
  (Rendering|SetVisibility (Variables|Default|GetSpotLight) false false)
  (Utilities|FlowControl|Delay 0.5)
  (bind _outactors (Actor|GetAllActorsOfClass "/Script/Engine.PlayerController"))
  (for (_ _array_index) _outactors
    (CameraFades|StartCameraFade (Game|GetPlayerCameraManager _array_index) 0.0 1.0 0.3 "(R=0.000000,G=0.000000,B=0.000000,A=1.000000)" true true))
  (Utilities|FlowControl|Delay 0.4)
  (for _array_element _outactors
    (bind _returnvalue (UserInterface|CreateWidget "/Game/Teapot_Content/Blueprints/Teapot_Victory_Widget.Teapot_Victory_Widget_C" _array_element))
    (UserInterface|Viewport|AddtoViewport _returnvalue 0)))

(fn ConstructionScript)