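; Two-holster weapon inventory screen that displays and stores the player's weapons as classes in the Teapot_PlayerController Inventory array.
; BeginPlay spawns each stored class at a holster, with physics off and query-only collision.
; Overlapping an empty holster box with an un-stored Teapot_Weapon_interface actor records its class, then flags, detaches and snaps it into place.
; Destruction removes the tracked actors but leaves the controller's array intact, so the next screen can rebuild them.
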(event OnComponentBeginOverlap(LeftHolsterBox)
  (params (OverlappedComponent :type Primitive%20Component%20Object%20Reference) (OtherActor :type Actor%20Object%20Reference) (OtherComp :type Primitive%20Component%20Object%20Reference) (OtherBodyIndex :type Integer) (bFromSweep :type Boolean) (SweepResult :type Hit%20Result%20Structure%20%28by%20ref%29))
  (if (Utilities|DoesObjectImplementInterface OtherActor "/Game/Teapot_Content/Blueprints/Teapot_Weapon_interface.Teapot_Weapon_interface_C")
    (bind _ininventory_ (Class|TeapotWeaponInterface|GetinInventory?(Message) OtherActor))
    (if (not _ininventory_)
      (bind _asteapot_player_controller (Utilities|Casting|CastToTeapot_PlayerController (Game|GetPlayerController 0)))
      (if (not (Utilities|IsValidClass (Utilities|Array|Get(acopy) (Variables|/Game/Teapot_Content/Blueprints/Teapot_PlayerController.Teapot_PlayerController_C|GetInventory _asteapot_player_controller))))
        (Utilities|Array|SetArrayElem (Variables|/Game/Teapot_Content/Blueprints/Teapot_PlayerController.Teapot_PlayerController_C|GetInventory _asteapot_player_controller) 0 (Utilities|GetClass OtherActor))
        (Utilities|Array|Add (Variables|Default|GetSpawnedActors) OtherActor)
        (bind _asstatic_mesh_actor (Utilities|Casting|CastToStaticMeshActor OtherActor))
        (Physics|SetSimulatePhysics (Variables|/Script/Engine.StaticMeshActor|GetStaticMeshComponent _asstatic_mesh_actor) false)
        (Collision|SetCollisionEnabled (Variables|/Script/Engine.StaticMeshActor|GetStaticMeshComponent _asstatic_mesh_actor) "QueryOnly")
        (Class|TeapotWeaponInterface|Setinventoryindex(Message) OtherActor)
        (Class|TeapotWeaponInterface|SetinInventory?(Message) OtherActor true)
        (Transformation|DetachFromActor OtherActor "KeepRelative" "KeepRelative" "KeepRelative")
        (Transformation|SetActorLocation OtherActor (Transformation|GetWorldLocation (Variables|Default|GetLeftHolsterBox)) false false)))))

(event OnComponentBeginOverlap(RightHolsterBox)
  (params (OverlappedComponent :type Primitive%20Component%20Object%20Reference) (OtherActor :type Actor%20Object%20Reference) (OtherComp :type Primitive%20Component%20Object%20Reference) (OtherBodyIndex :type Integer) (bFromSweep :type Boolean) (SweepResult :type Hit%20Result%20Structure%20%28by%20ref%29))
  (if (Utilities|DoesObjectImplementInterface OtherActor "/Game/Teapot_Content/Blueprints/Teapot_Weapon_interface.Teapot_Weapon_interface_C")
    (bind _ininventory_ (Class|TeapotWeaponInterface|GetinInventory?(Message) OtherActor))
    (if (not _ininventory_)
      (bind _asteapot_player_controller (Utilities|Casting|CastToTeapot_PlayerController (Game|GetPlayerController 0)))
      (if (not (Utilities|IsValidClass (Utilities|Array|Get(acopy) (Variables|/Game/Teapot_Content/Blueprints/Teapot_PlayerController.Teapot_PlayerController_C|GetInventory _asteapot_player_controller) 1)))
        (Utilities|Array|SetArrayElem (Variables|/Game/Teapot_Content/Blueprints/Teapot_PlayerController.Teapot_PlayerController_C|GetInventory _asteapot_player_controller) 1 (Utilities|GetClass OtherActor))
        (Utilities|Array|Add (Variables|Default|GetSpawnedActors) OtherActor)
        (bind _asstatic_mesh_actor (Utilities|Casting|CastToStaticMeshActor OtherActor))
        (CallFunction|ServerSimulatePhysics)
        (Class|TeapotWeaponInterface|Setinventoryindex(Message) OtherActor 1)
        (Class|TeapotWeaponInterface|SetinInventory?(Message) OtherActor true)
        (Transformation|DetachFromActor OtherActor "KeepRelative" "KeepRelative" "KeepRelative")
        (Transformation|SetActorLocation OtherActor (Transformation|GetWorldLocation (Variables|Default|GetRightHolsterBox)) false false)))))

(event Custom|ServerSimulatePhysics
  (Physics|SetSimulatePhysics (Variables|/Script/Engine.StaticMeshActor|GetStaticMeshComponent (stale OnComponentBeginOverlap(RightHolsterBox) _asstatic_mesh_actor)) false)
  (Collision|SetCollisionEnabled (Variables|/Script/Engine.StaticMeshActor|GetStaticMeshComponent (stale OnComponentBeginOverlap(RightHolsterBox) _asstatic_mesh_actor)) "QueryOnly"))

(event EventBeginPlay
  (bind _asteapot_player_controller (Utilities|Casting|CastToTeapot_PlayerController (Game|GetPlayerController 0)))
  (for (_array_element _array_index) (Variables|/Game/Teapot_Content/Blueprints/Teapot_PlayerController.Teapot_PlayerController_C|GetInventory _asteapot_player_controller)
    (if (Utilities|IsValidClass _array_element)
      (bind _returnvalue (Game|SpawnActorfromClass _array_element (Math|Transform|MakeTransform (Transformation|GetWorldLocation (Utilities|Array|Get(acopy) (Utilities|Array|MakeArray (Variables|Default|GetLeftHolster) (Variables|Default|GetRightHolster)) _array_index))) "Undefined" 0 0))
      (Utilities|Array|Add (Variables|Default|GetSpawnedActors) _returnvalue)
      (Class|TeapotWeaponInterface|SetinInventory?(Message) _returnvalue true)
      (Class|TeapotWeaponInterface|Setinventoryindex(Message) _returnvalue _array_index)
      (bind _asstatic_mesh_actor (Utilities|Casting|CastToStaticMeshActor _returnvalue))
      (Physics|SetSimulatePhysics (Variables|/Script/Engine.StaticMeshActor|GetStaticMeshComponent _asstatic_mesh_actor) false)
      (Collision|SetCollisionEnabled (Variables|/Script/Engine.StaticMeshActor|GetStaticMeshComponent _asstatic_mesh_actor) "QueryOnly"))))

(event EventDestroyed
  (bind _spawnedactors (Variables|Default|GetSpawnedActors))
  (for _array_element _spawnedactors
    (Actor|DestroyActor _array_element))
  (Utilities|Array|Clear _spawnedactors))

(fn ConstructionScript)