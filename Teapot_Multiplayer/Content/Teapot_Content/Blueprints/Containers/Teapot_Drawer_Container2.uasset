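; Searchable drawer container for a turn-based VR game that spawns a random item or zombie when searched.
; On BeginPlay it stores the overlapped tile; server-side pickup allows one search, on the player's turn, costing an action.
; Spawns draw from GameState's PossibleItems, re-rolling between type check and spawn; zombies land on the tile and raise its cost, items at a spawn point.
; Door-dragging logic is unused.
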(event Custom|Spawn%20Actor%20on%20server
  (bind _itemspawnlocationr (Variables|Default|GetItemSpawnlocationR))
  (bind _returnvalue (Transformation|GetWorldLocation _itemspawnlocationr))
  ;[1 1 1] Spawns actor on server
  (bind _asteapot_game_state (Utilities|Casting|CastToTeapot_GameState (Game|GetGameState)))
  (if (== (Utilities|Array|Get(acopy) (Variables|/Game/Teapot_Content/Blueprints/Teapot_GameState.Teapot_GameState_C|GetPossibleItems _asteapot_game_state) (Math|Random|RandomInteger (Utilities|Array|Length (Variables|/Game/Teapot_Content/Blueprints/Teapot_GameState.Teapot_GameState_C|GetPossibleItems _asteapot_game_state)))) "/Game/Teapot_Content/Blueprints/Teapot_Zombie_Standard.Teapot_Zombie_Standard_C")
    (bind _returnvalue_2 (Game|SpawnActorfromClass (Utilities|Array|Get(acopy) (Variables|/Game/Teapot_Content/Blueprints/Teapot_GameState.Teapot_GameState_C|GetPossibleItems _asteapot_game_state) (Math|Random|RandomInteger (Utilities|Array|Length (Variables|/Game/Teapot_Content/Blueprints/Teapot_GameState.Teapot_GameState_C|GetPossibleItems _asteapot_game_state)))) (Math|Conversions|ToTransform(Vector) (+ (Transformation|GetWorldLocation (Variables|/Game/Teapot_Content/Blueprints/Teapot_Tile.Teapot_Tile_C|GetBox (Variables|Default|GetCurrentTile))) "0, 0,120.000000")) "AlwaysSpawn" 0 0))
    (bind _asteapot_zombie_standard (Utilities|Casting|CastToTeapot_Zombie_Standard _returnvalue_2))
    (Variables|/Game/Teapot_Content/Blueprints/Teapot_Zombie_Standard.Teapot_Zombie_Standard_C|SetCurrentTile _asteapot_zombie_standard (Variables|Default|GetCurrentTile))
    (Math|Integer|IncrementInt (Variables|/Game/Teapot_Content/Blueprints/Teapot_Tile.Teapot_Tile_C|GetActionCost (Variables|Default|GetCurrentTile)))
    (else
      (bind _returnvalue_3 (Game|SpawnActorfromClass (Utilities|Array|Get(acopy) (Variables|/Game/Teapot_Content/Blueprints/Teapot_GameState.Teapot_GameState_C|GetPossibleItems _asteapot_game_state) (Math|Random|RandomInteger (Utilities|Array|Length (Variables|/Game/Teapot_Content/Blueprints/Teapot_GameState.Teapot_GameState_C|GetPossibleItems _asteapot_game_state)))) (Math|Conversions|ToTransform(Vector) _returnvalue) "AlwaysSpawn" 0 0))
      (Transformation|SetActorLocation _returnvalue_3 _returnvalue false false))))

(event Custom|serverTic
  ;[1 1 1] Not in use, used for moving door
)

(event EventBeginPlay
  (bind _array_element (Utilities|Array|ForEachLoopwithBreak (Collision|GetOverlappingActors (Variables|Default|GetWardrobeBase) "/Game/Teapot_Content/Blueprints/Teapot_Tile.Teapot_Tile_C" :!class /Script/Engine.PrimitiveComponent) :!label _label)
    (:LoopBody
      (bind _asteapot_tile (Utilities|Casting|CastToTeapot_Tile _array_element))
      (Variables|Default|SetCurrentTile _asteapot_tile)
      (goto _label Break))))

(event EventTeapotDrop
  ;[1 1 1] Not in use, used for moving door
)

(event EventTeapotPickup
  (params (AttachTo :type Scene%20Component%20Object%20Reference) (PlayerIndex :type Integer))
  (bind _returnvalue (Components|GetOwner AttachTo))
  ;[1 1 1] On interaction (runs on server)
  (bind _asteapot_motion_controller (Utilities|Casting|CastToTeapot_MotionController _returnvalue))
  (Variables|/Game/Teapot_Content/Blueprints/Teapot_MotionController.Teapot_MotionController_C|SetAttachedActor _asteapot_motion_controller 0)
  (if (not (Variables|Default|GetisSearched))
    (bind _asteapot_vrpawn (Utilities|Casting|CastToTeapot_VRPawn (Actor|GetAttachParentActor _returnvalue)))
    (bind _asteapot_player_controller (Utilities|Casting|CastToTeapot_PlayerController (Pawn|GetController _asteapot_vrpawn)))
    (bind _asteapot_game_mode (Utilities|Casting|CastToTeapot_GameMode (Game|GetGameMode)))
    (if (== (Variables|/Game/Teapot_Content/Blueprints/Teapot_GameMode.Teapot_GameMode_C|GetTurnIndex _asteapot_game_mode) (Variables|/Game/Teapot_Content/Blueprints/Teapot_PlayerController.Teapot_PlayerController_C|GetPlayerIndex _asteapot_player_controller))
      (Default|ReduceActionsClient _asteapot_vrpawn 1)
      (CallFunction|SpawnActoronServer)
      (Variables|Default|SetisSearched true))))

(fn ConstructionScript)