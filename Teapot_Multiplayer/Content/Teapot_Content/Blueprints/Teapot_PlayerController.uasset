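; Player controller for Teapot's turn-based multiplayer VR game, handling session hotkeys and turn passing.
; Input actions host or join the first LAN session found through the GameInstance, and either leave to the lobby or quit, depending on its state.
; T or left grip checks the GameState turn index, requests GameMode's next turn, then resets PlayerState actions and updates the VR pawn's text.
; Debug keys print turn and action values.
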(event Custom|AskForNextTurn
  ;[1 1 1] Ask server to switch turn
  (bind _asteapot_game_mode (Utilities|Casting|CastToTeapot_GameMode (Game|GetGameMode))
    (:then
      (if (== (Variables|Default|GetPlayerIndex) (Variables|/Game/Teapot_Content/Blueprints/Teapot_GameMode.Teapot_GameMode_C|GetTurnIndex _asteapot_game_mode))
        (Default|NextTurn _asteapot_game_mode)
        (Development|PrintString "\"Next Turn\" Successful" true true "(R=0.000000,G=0.660000,B=1.000000,A=1.000000)" 5.0)
        (else
          (Development|PrintString "\"Next Turn\" failed" true true "(R=0.000000,G=0.660000,B=1.000000,A=1.000000)" 5.0))))
    (:CastFailed
      (Development|PrintString "Cast Failed to gamemode in ask for nextturn" true true "(R=0.000000,G=0.660000,B=1.000000,A=1.000000)" 1e+01))))

(event EventBeginPlay)

(event EventTick
  (params (DeltaSeconds :type Float%20%28single-precision%29)))

(event Input|ActionEvents|InputActionJoinGameKey
  (params (Key :type Key%20Structure :default "AnyKey"))
  (:Pressed
    (Development|PrintString "j")
    (Utilities|Array|Clear (Variables|Default|GetFoundSession))
    (bind _results (|FindSessions (Game|GetPlayerController 0) 20 true)
      (:OnSuccess
        (bind _output_get (Variables|Default|SetFoundSession _results))
        (bind _array_element (Utilities|Array|ForEachLoopwithBreak _output_get :!label _label)
          (:LoopBody
            (Variables|Default|SetSessionFound true)
            (Variables|Default|SetAvailableSession _array_element)
            (goto _label Break))
          (:Completed
            (if (Variables|Default|GetSessionFound)
              (bind _asteapot_game_instance (Utilities|Casting|CastToTeapot_GameInstance (Game|GetGameInstance))
                (:then
                  (Default|JoinGameEvent _asteapot_game_instance (Variables|Default|GetAvailableSession)))
                (:CastFailed
                  (Development|PrintString "Error session found but not valid")))))))
      (:OnFailure
        (Development|PrintString "Error Finding session")))))

(event Input|ActionEvents|InputActionHostGameKey
  (params (Key :type Key%20Structure :default "AnyKey"))
  ;[1 1 1] Press H to host game session
  (:Pressed
    (Development|PrintString "H Pressed")
    (bind _asteapot_game_instance (Utilities|Casting|CastToTeapot_GameInstance (Game|GetGameInstance))
      (:then
        (Default|HostGameEvent _asteapot_game_instance))
      (:CastFailed
        (Development|PrintString "Host cast failed")))))

(event Input|ActionEvents|InputActionQuitGameKey
  (params (Key :type Key%20Structure :default "AnyKey"))
  ;[1 1 1] Press Escape to Quit
  (:Pressed
    (bind _asteapot_game_instance (Utilities|Casting|CastToTeapot_GameInstance (Game|GetGameInstance)))
    (bind _currentstate (Default|GetCurrentState _asteapot_game_instance))
    (if (Utilities|Enum|Equal(Enum) "NewEnumerator1" _currentstate)
      (|DestroySession (Game|GetPlayerController 0)
        (:then
          (Game|OpenLevel(byName) "Teapot_Level_Lobby")
          (bind _asteapot_game_instance_2 (Utilities|Casting|CastToTeapot_GameInstance (Game|GetGameInstance)))
          (Variables|/Game/Teapot_Content/Blueprints/Teapot_GameInstance.Teapot_GameInstance_C|SetCurrentState _asteapot_game_instance_2 "NewEnumerator0"))
        (:OnSuccess
          (Development|PrintString "Succeeded Destroying session"))
        (:OnFailure
          (Development|PrintString "Failed Destroying Session")))
      (else
        (Game|QuitGame 0 "Quit")))))

(event Input|ActionEvents|InputActionDebugGameKey
  (params (Key :type Key%20Structure :default "AnyKey"))
  ;[1 1 1] "0 Pressed"
  (:Pressed
    (Development|PrintString "0 Pressed!")))

(event Input|KeyboardEvents|T
  (params (Key :type Key%20Structure :default "AnyKey"))
  ;[1 1 1] Press T/Grip (L) to switch turn
  (:Pressed
    (bind _asteapot_player_state (Utilities|Casting|CastToTeapot_PlayerState (Variables|GetPlayerState)))
    (bind _asteapot_game_state (Utilities|Casting|CastToTeapot_GameState (Game|GetGameState)))
    (if (== (Variables|/Game/Teapot_Content/Blueprints/Teapot_GameState.Teapot_GameState_C|GetTurnIndex _asteapot_game_state) (Variables|Default|GetPlayerIndex))
      (CallFunction|AskforNextTurn)
      (Variables|/Game/Teapot_Content/Blueprints/Teapot_PlayerState.Teapot_PlayerState_C|SetRemainingActions _asteapot_player_state (Variables|/Game/Teapot_Content/Blueprints/Teapot_PlayerState.Teapot_PlayerState_C|GetNewTurnActions _asteapot_player_state))
      (bind _asteapot_vrpawn (Utilities|Casting|CastToTeapot_VRPawn (Pawn|GetControlledPawn)))
      (Default|UpdateActionsTextClient _asteapot_vrpawn))))

(event Input|KeyboardEvents|N
  (params (Key :type Key%20Structure :default "AnyKey"))
  (:Pressed
    (bind _asteapot_player_state (Utilities|Casting|CastToTeapot_PlayerState (Variables|GetPlayerState)))
    (Development|PrintString (Utilities|String|ToString(Integer) (Variables|/Game/Teapot_Content/Blueprints/Teapot_PlayerState.Teapot_PlayerState_C|GetRemainingActions _asteapot_player_state)) true true "(R=0.093309,G=0.250000,B=0.021708,A=1.000000)" 1e+01)))

(event Input|KeyboardEvents|M
  (params (Key :type Key%20Structure :default "AnyKey"))
  (:Pressed
    (Development|PrintString (Utilities|String|ToString(Integer) (Variables|Default|GetPlayerIndex)) true true "(R=1.000000,G=0.790984,B=0.000000,A=1.000000)" 1e+01)
    (bind _asteapot_game_state (Utilities|Casting|CastToTeapot_GameState (Game|GetGameState))
      (:then
        (Development|PrintString (Utilities|String|ToString(Integer) (Variables|/Game/Teapot_Content/Blueprints/Teapot_GameState.Teapot_GameState_C|GetTurnIndex _asteapot_game_state)) true true "(R=1.000000,G=0.000000,B=0.983937,A=1.000000)" 1e+01))
      (:CastFailed
        (Development|PrintString "GameModeStateFail" true true "(R=0.000000,G=1.000000,B=0.374051,A=1.000000)" 1e+01)))))

(event Input|KeyboardEvents|MotionControllerLeftGrip1
  (params (Key :type Key%20Structure :default "AnyKey"))
  ;[1 1 1] Press T/Grip (L) to switch turn
  (:Pressed
    (bind _asteapot_player_state (Utilities|Casting|CastToTeapot_PlayerState (Variables|GetPlayerState)))
    (bind _asteapot_game_state (Utilities|Casting|CastToTeapot_GameState (Game|GetGameState)))
    (if (== (Variables|/Game/Teapot_Content/Blueprints/Teapot_GameState.Teapot_GameState_C|GetTurnIndex _asteapot_game_state) (Variables|Default|GetPlayerIndex))
      (CallFunction|AskforNextTurn)
      (Variables|/Game/Teapot_Content/Blueprints/Teapot_PlayerState.Teapot_PlayerState_C|SetRemainingActions _asteapot_player_state (Variables|/Game/Teapot_Content/Blueprints/Teapot_PlayerState.Teapot_PlayerState_C|GetNewTurnActions _asteapot_player_state))
      (bind _asteapot_vrpawn (Utilities|Casting|CastToTeapot_VRPawn (Pawn|GetControlledPawn)))
      (Default|UpdateActionsTextClient _asteapot_vrpawn))))

(fn ConstructionScript)