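; Enemy spawner actor that keeps one unit of a configurable class alive at its location.
; It spawns the unit on BeginPlay at the spawner's position with zero rotation and unit scale, and stores a reference to it.
; Tick polls that reference and, once it is invalid, runs a Delay of the configured spawn timer before calling Respawn to spawn a replacement.
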(event Custom|Respawn
  (bind _returnvalue (Game|SpawnActorfromClass (Variables|Default|GetclassToSpawn) (Math|Transform|MakeTransform (Transformation|GetActorLocation)) "Undefined" 0 0))
  (Variables|Default|SetSpawnedUnit _returnvalue))

(event EventBeginPlay
  (bind _returnvalue (Game|SpawnActorfromClass (Variables|Default|GetclassToSpawn) (Math|Transform|MakeTransform (Transformation|GetActorLocation)) "Undefined" 0 0))
  (Variables|Default|SetSpawnedUnit _returnvalue))

(event EventTick
  (params (DeltaSeconds :type Float%20%28single-precision%29))
  (if (not (Utilities|IsValid (Variables|Default|GetSpawnedUnit)))
    (Utilities|FlowControl|Delay (Variables|Default|GetSpawntimer))
    (CallFunction|Respawn)))

(fn ConstructionScript)