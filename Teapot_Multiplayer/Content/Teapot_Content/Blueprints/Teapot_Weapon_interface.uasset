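; Blueprint interface for weapons, declaring what a weapon exposes to the code that uses it.
; Query functions report whether the weapon is melee, throwable, silent or able to break doors, along with its damage.
; Further functions get and set inventory state, set the inventory index, and declare hit and shoot calls.
; All functions are stubs with empty bodies or default returns, leaving behavior to implementing Blueprints.
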(fn GetCanbreakdoor
  (return false))

(fn GetisMelee
  (return false))

(fn GetisThrowable
  (return false))

(fn GetisSilent
  (return false))

(fn Weaponhit?
  (return 0))

(fn GetDamage
  (return 0))

(fn SetinInventory?
  (params (inInventory? :type Boolean)))

(fn GetinInventory?
  (return false))

(fn Setinventoryindex
  (params (Inventoryindex :type Integer)))

(fn Shoot!)