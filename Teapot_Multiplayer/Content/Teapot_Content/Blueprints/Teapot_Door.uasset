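; Breakable door actor for the Teapot game, destroyed with a break sound when a capable actor touches it during the player's turn.
; Box overlap asks the other actor whether it can break doors, then checks turn state on Teapot_GameState before calling BreakDoorServer.
; Failed checks only print debug messages; action cost is a noted TODO, and CheckisDoorbreak is a stub returning false.
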(event OnComponentBeginOverlap(Box)
  (params (OverlappedComponent :type Primitive%20Component%20Object%20Reference) (OtherActor :type Actor%20Object%20Reference) (OtherComp :type Primitive%20Component%20Object%20Reference) (OtherBodyIndex :type Integer) (bFromSweep :type Boolean) (SweepResult :type Hit%20Result%20Structure%20%28by%20ref%29))
  (bind _canbreakdoor (Class|TeapotWeaponInterface|GetCanbreakdoor(Message) OtherActor))
  (if _canbreakdoor
    (bind _asteapot_game_state (Utilities|Casting|CastToTeapot_GameState (Game|GetGameState)))
    ;[1 1 1] Also check for actions and remove one
    (bind _ismyturn (Default|IsMyTurn _asteapot_game_state))
    (if _ismyturn
      ;[1 1 1] Is this correct?
      (CallFunction|BreakDoorServer)
      (else
        (Development|PrintString "Debug msg: 
It is not your turn," true true "(R=0.000000,G=0.660000,B=1.000000,A=1.000000)" 1e+01)))
    (else
      (Development|PrintString "Debug msg: 
Weapon can not break doors." true true "(R=0.000000,G=0.660000,B=1.000000,A=1.000000)" 1e+01))))

(event Custom|BreakDoorServer
  ;[1 1 1] Is this correct?
  (Actor|DestroyActor)
  (Audio|PlaySound2D "/Game/Teapot_Content/Sounds/Teapot_breakdoor.Teapot_breakdoor"))

(fn ConstructionScript)

(fn CheckisDoorbreak
  (return false))