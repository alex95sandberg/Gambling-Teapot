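; Searchable wardrobe container for a turn-based VR game that yields a victory weapon.
; TeapotPickup runs on the server, clears the motion controller's attached actor, then checks that the container is unsearched and the player has the turn and an action left.
; A valid search spends one action, marks the container searched and spawns Teapot_Victory_Weapon at the item spawn point.
; Hand-driven door movement remains as disconnected, unused logic.
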(event Custom|Spawn%20Actor%20on%20server
  (bind _itemspawnlocationr (Variables|Default|GetItemSpawnlocationR))
  (bind _returnvalue (Transformation|GetWorldLocation _itemspawnlocationr))
  ;[1 1 1] Spawns actor on server
  (Utilities|Casting|CastToTeapot_GameState (Game|GetGameState))
  (bind _returnvalue_2 (Game|SpawnActorfromClass "/Game/Teapot_Content/Blueprints/Weapons/Teapot_Victory_Weapon.Teapot_Victory_Weapon_C" (Math|Conversions|ToTransform(Vector) _returnvalue) "AlwaysSpawn" 0 0))
  (Transformation|SetActorLocation _returnvalue_2 _returnvalue false false))

(event Custom|serverTic
  ;[1 1 1] Not in use, used for moving door
)

(event EventTeapotDrop
  ;[1 1 1] Not in use, used for moving door
)

(event EventTeapotPickup
  (params (AttachTo :type Scene%20Component%20Object%20Reference) (PlayerIndex :type Integer))
  (bind _returnvalue (Components|GetOwner AttachTo))
  ;[1 1 1] On interaction (runs on server)
  (bind _asteapot_motion_controller (Utilities|Casting|CastToTeapot_MotionController _returnvalue))
  (Variables|/Game/Teapot_Content/Blueprints/Teapot_MotionController.Teapot_MotionController_C|SetAttachedActor _asteapot_motion_controller 0)
  (if (not (Variables|Default|GetisSearched))
    (bind _asteapot_vrpawn (Utilities|Casting|CastToTeapot_VRPawn (Actor|GetAttachParentActor _returnvalue)))
    (bind _asteapot_player_controller (Utilities|Casting|CastToTeapot_PlayerController (Pawn|GetController _asteapot_vrpawn)))
    (bind _asteapot_game_mode (Utilities|Casting|CastToTeapot_GameMode (Game|GetGameMode)))
    (bind _asteapot_player_state (Utilities|Casting|CastToTeapot_PlayerState (Variables|/Script/Engine.Controller|GetPlayerState _asteapot_player_controller)))
    (if (and (== (Variables|/Game/Teapot_Content/Blueprints/Teapot_GameMode.Teapot_GameMode_C|GetTurnIndex _asteapot_game_mode) (Variables|/Game/Teapot_Content/Blueprints/Teapot_PlayerController.Teapot_PlayerController_C|GetPlayerIndex _asteapot_player_controller)) (>= (Variables|/Game/Teapot_Content/Blueprints/Teapot_PlayerState.Teapot_PlayerState_C|GetRemainingActions _asteapot_player_state) 1))
      (Default|ReduceActionsClient _asteapot_vrpawn 1)
      (Variables|Default|SetisSearched true)
      (CallFunction|SpawnActoronServer))))

(fn ConstructionScript)