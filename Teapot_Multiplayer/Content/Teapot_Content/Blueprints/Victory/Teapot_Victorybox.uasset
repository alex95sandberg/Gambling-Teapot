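; Victory box for the VR teapot game that triggers the win sequence when a Teapot_VictoryItem overlaps its Box.
; On overlap it clears AttachedActor on any motion controller found as attach parent, destroys the item and reveals a static battery.
; Timed delays then turn one spotlight on and another off before the victory text is shown on every Teapot_VRPawn.
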(event OnComponentBeginOverlap(Box)
  (params (OverlappedComponent :type Primitive%20Component%20Object%20Reference) (OtherActor :type Actor%20Object%20Reference) (OtherComp :type Primitive%20Component%20Object%20Reference) (OtherBodyIndex :type Integer) (bFromSweep :type Boolean) (SweepResult :type Hit%20Result%20Structure%20%28by%20ref%29))
  (bind _asteapot_victory_item (Utilities|Casting|CastToTeapot_VictoryItem OtherActor))
  (bind _asteapot_motion_controller (Utilities|Casting|CastToTeapot_MotionController (Actor|GetAttachParentActor))
    (:then
      (Variables|/Game/Teapot_Content/Blueprints/Teapot_MotionController.Teapot_MotionController_C|SetAttachedActor _asteapot_motion_controller 0))
    (:CastFailed
      _))
  (Actor|DestroyActor _asteapot_victory_item)
  (Rendering|SetVisibility (Variables|Default|GetStaticBattery) true false)
  (Utilities|FlowControl|Delay 1.0)
  (Rendering|SetVisibility (Variables|Default|GetSpotLight1) true true)
  (Utilities|FlowControl|Delay 1.0)
  (Rendering|SetVisibility (Variables|Default|GetSpotLight) false false)
  (bind _outactors (Actor|GetAllActorsOfClass "/Game/Teapot_Content/Blueprints/Teapot_VRPawn.Teapot_VRPawn_C"))
  (for _array_element _outactors
    (Rendering|SetVisibility (Variables|/Game/Teapot_Content/Blueprints/Teapot_VRPawn.Teapot_VRPawn_C|GetVictroyText _array_element) true false)))

(fn ConstructionScript)