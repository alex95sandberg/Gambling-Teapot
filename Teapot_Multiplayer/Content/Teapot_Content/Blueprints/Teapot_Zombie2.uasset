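; Tile-based zombie that, on each LerpMovement call, steps one tile toward the noisiest Teapot_Tile on the map.
; FindShortestPath targets all tiles sharing the highest noise, then FSPRecursive searches connected tiles depth-first, keeping the path with fewest tiles.
; A Timeline lerps the zombie to the next tile with walk and idle animations, then shifts its action cost and fog registration between tiles.
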(event Custom|LerpMovement
  (bind _returnvalue (Transformation|GetActorLocation))
  (bind _shortestpath (Variables|Default|GetShortestPath))
  (bind _item (Utilities|Array|Get(acopy) _shortestpath 1))
  (bind _z (Math|Vector|BreakVector _returnvalue))
  (bind _returnvalue_2 (Transformation|GetActorLocation _item))
  (bind (_x _y) (Math|Vector|BreakVector _returnvalue_2))
  (bind _returnvalue_3 (Math|Vector|MakeVector _x _y _z))
  (Development|PrintString "N")
  (bind _asteapot_tile (Utilities|Casting|CastToTeapot_Tile (Variables|Default|GetCurrentTile)))
  (CallFunction|FindShortestPath _asteapot_tile)
  (if (!= _item 0)
    ;[1 1 1] Lerp to new location
    (Transformation|SetActorRotation (Math|Rotator|FindLookatRotation (Math|Vector|MakeVector (.X (Math|Vector|BreakVector (Transformation|GetActorLocation (Variables|Default|GetCurrentTile)))) (.Y (Math|Vector|BreakVector (Transformation|GetActorLocation (Variables|Default|GetCurrentTile)))) _z) _returnvalue_3))
    (Components|Animation|PlayAnimation (Variables|Character|GetMesh) "/Game/Mannequin/Animations/ThirdPersonWalk.ThirdPersonWalk" true)
    (bind _alpha (Timeline|Timeline_0 PlayFromStart)
      (:Update
        (Transformation|SetActorLocation (Math|Vector|Lerp(Vector) (Math|Vector|MakeVector (.X (Math|Vector|BreakVector (Transformation|GetActorLocation (Variables|Default|GetCurrentTile)))) (.Y (Math|Vector|BreakVector (Transformation|GetActorLocation (Variables|Default|GetCurrentTile)))) _z) _returnvalue_3 _alpha) false false))
      (:Finished
        (Components|Animation|PlayAnimation (Variables|Character|GetMesh) "/Game/Mannequin/Animations/ThirdPersonIdle.ThirdPersonIdle" true)
        ;[1 1 1] When the zombie have succesfully moved to it's new location
        (bind _result (Math|Integer|DecrementInt (Variables|/Game/Teapot_Content/Blueprints/Teapot_Tile.Teapot_Tile_C|GetActionCost _asteapot_tile))
          (:%20%20
            (Variables|/Game/Teapot_Content/Blueprints/Teapot_Tile.Teapot_Tile_C|SetActionCost _asteapot_tile _result)
            (Utilities|Array|RemoveItem (Variables|/Game/Teapot_Content/Blueprints/Teapot_Tile.Teapot_Tile_C|GetFogAffectedActors _asteapot_tile) self)
            (bind _output_get (Variables|Default|SetCurrentTile _item))
            (bind _asteapot_tile_2 (Utilities|Casting|CastToTeapot_Tile _output_get))
            (bind _result_2 (Math|Integer|IncrementInt (Variables|/Game/Teapot_Content/Blueprints/Teapot_Tile.Teapot_Tile_C|GetActionCost _asteapot_tile_2))
              (:%20%20
                (Variables|/Game/Teapot_Content/Blueprints/Teapot_Tile.Teapot_Tile_C|SetActionCost _asteapot_tile_2 _result_2)
                (Utilities|Array|Add (Variables|/Game/Teapot_Content/Blueprints/Teapot_Tile.Teapot_Tile_C|GetFogAffectedActors _asteapot_tile_2) self)))))))))

(event Collision|EventActorBeginOverlap
  (params (OtherActor :type Actor%20Object%20Reference)))

(fn ConstructionScript)

(fn FindShortestPath
  (params (CurrentTile :type Teapot%20Tile%20Object%20Reference))
  (bind _path (LocalVariables|GetPath))
  (bind _path_2 (LocalVariables|GetPath))
  (bind _path_3 (LocalVariables|GetPath))
  (bind _targettiles (Variables|Default|GetTargetTiles))
  ;[1 1 1] Reset all values
  (Utilities|Array|Clear (Variables|Default|GetShortestPath))
  (Variables|Default|SetHighestNoise 0)
  (Utilities|Array|Clear (Variables|Default|GetTargetTiles))
  (Utilities|Array|Clear _path)
  (Utilities|Array|Add _path CurrentTile)
  ;[1 1 1] Find the tiles with the highest noise and make them the targets
  (bind _outactors (Actor|GetAllActorsOfClass "/Game/Teapot_Content/Blueprints/Teapot_Tile.Teapot_Tile_C"))
  (for _array_element _outactors
    (if (== (Variables|/Game/Teapot_Content/Blueprints/Teapot_Tile.Teapot_Tile_C|GetNoise _array_element) (Variables|Default|GetHighestNoise))
      (Utilities|Array|Add _targettiles _array_element :!label _label)
      (Variables|Default|SetHighestNoise (Variables|/Game/Teapot_Content/Blueprints/Teapot_Tile.Teapot_Tile_C|GetNoise _array_element))
      (elif (> (Variables|/Game/Teapot_Content/Blueprints/Teapot_Tile.Teapot_Tile_C|GetNoise _array_element) (Variables|Default|GetHighestNoise))
        (Utilities|Array|Clear _targettiles)
        (goto _label))))
  (bind _array_element_2 (Utilities|Array|ForEachLoopwithBreak (Variables|/Game/Teapot_Content/Blueprints/Teapot_Tile.Teapot_Tile_C|GetConnectedTiles CurrentTile) :!label _label_2)
    (:LoopBody
      (bind _asteapot_tile (Utilities|Casting|CastToTeapot_Tile _array_element_2))
      (if (Utilities|Array|ContainsItem (Variables|Default|GetTargetTiles) _asteapot_tile)
        ;[1 1 1] We've found a path
        (Utilities|Array|Add _path_3 _asteapot_tile)
        (Variables|Default|SetShortestPath _path_3)
        (goto _label_2 Break)
        (elif (not (Utilities|Array|ContainsItem _path_2 _asteapot_tile))
          (CallFunction|FSPRecursive _asteapot_tile _path_2) ; Start to recursively check all tiles for a path
        )))
    (:Completed
      (Development|PrintString "Completed pathfinding"))))

(fn FSPRecursive
  (params (CurrentTile :type Teapot%20Tile%20Object%20Reference) (Path :type Array%20of%20Teapot%20Tile%20Object%20References))
  (bind _output_get (LocalVariables|SetTempPath Path))
  (Utilities|Array|Add _output_get CurrentTile)
  (for _array_element (Variables|/Game/Teapot_Content/Blueprints/Teapot_Tile.Teapot_Tile_C|GetConnectedTiles CurrentTile)
    (bind _asteapot_tile (Utilities|Casting|CastToTeapot_Tile _array_element))
    (if (Utilities|Array|ContainsItem (Variables|Default|GetTargetTiles) _asteapot_tile)
      (Utilities|Array|Add (LocalVariables|GetTempPath) _asteapot_tile)
      ;[1 1 1] A path to the target has been found, check if it is the shortest so far
      (if (or (<= (Utilities|Array|Length (LocalVariables|GetTempPath)) (Utilities|Array|Length (Variables|Default|GetShortestPath))) (== (Utilities|Array|Length (Variables|Default|GetShortestPath)) 0))
        (Variables|Default|SetShortestPath (LocalVariables|GetTempPath)))
      (elif (not (Utilities|Array|ContainsItem (LocalVariables|GetTempPath) _asteapot_tile))
        (CallFunction|FSPRecursive _asteapot_tile (LocalVariables|GetTempPath))))))