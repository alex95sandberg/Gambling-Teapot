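; Katana weapon actor for a turn-based zombie game, with pickup, drop and weapon-stat getters.
; Pickup attaches it to the given component, or, from inventory, spawns an attached replacement, updates the inventory and destroys itself.
; Overlapping a zombie on the player's turn spends an action and rolls d6s against Hitchance, flashing a green or red cube and destroying that zombie on any hit.
; Multi-zombie attack logic is an unused sketch.
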(event OnComponentBeginOverlap(StaticMeshComponent)
  (params (OverlappedComponent :type Primitive%20Component%20Object%20Reference) (OtherActor :type Actor%20Object%20Reference) (OtherComp :type Primitive%20Component%20Object%20Reference) (OtherBodyIndex :type Integer) (bFromSweep :type Boolean) (SweepResult :type Hit%20Result%20Structure%20%28by%20ref%29))
  ;[1 1 1] Can only hit one Zombie
  (bind _asteapot_zombie (Utilities|Casting|CastToTeapot_Zombie OtherActor))
  (bind _asteapot_game_state (Utilities|Casting|CastToTeapot_GameState (Game|GetGameState)))
  (bind _ismyturn (Default|IsMyTurn _asteapot_game_state))
  (if (Math|Boolean|ANDBoolean _ismyturn (Variables|WeaponProperties|GetisMelee) (not (Variables|Default|GetinInventory?)))
    (Variables|Default|SetDestroyActor _asteapot_zombie)
    (Default|ReduceRemainingActions _asteapot_game_state 1)
    (bind _hits (CallFunction|Weaponhit?))
    ;[1 1 1] Note
    (bind _returnvalue (Game|SpawnActorfromClass "/Game/Teapot_Content/Blueprints/Teapot_PickupCube.Teapot_PickupCube_C" (Math|Conversions|ToTransform(Vector) (+ (Transformation|GetActorLocation _asteapot_zombie) "0, 0,150.000000")) "AlwaysSpawn" 0 0))
    (Physics|SetSimulatePhysics (Variables|/Script/Engine.StaticMeshActor|GetStaticMeshComponent _returnvalue) false)
    (if (Utilities|Array|ContainsItem _hits true)
      (Rendering|Material|SetMaterial (Variables|/Script/Engine.StaticMeshActor|GetStaticMeshComponent _returnvalue) 0 "/Game/Teapot_Content/Materials/Teapot_Green.Teapot_Green")
      (Utilities|FlowControl|Delay 0.6)
      (CallFunction|DestroyZombieonServer)
      (else
        (Rendering|Material|SetMaterial (Variables|/Script/Engine.StaticMeshActor|GetStaticMeshComponent _returnvalue) 0 "/Game/Teapot_Content/Materials/Teapot_Red.Teapot_Red")
        (Utilities|FlowControl|Delay 0.6)))
    (Actor|DestroyActor _returnvalue)
    (Utilities|Array|Clear (Variables|Default|GetHit))
    (Variables|Default|SetDestroyActor 0)))

(event Custom|Make%20Serverweapon
  (bind _self self)
  ;[1 1 1] MP test
  (bind _returnvalue (Game|SpawnActorfromClass "Teapot_Katana_Weapon5_C" (Math|Transform|MakeTransform (Transformation|GetActorLocation _self) (Transformation|GetActorRotation _self)) "Undefined" 0 0))
  (Physics|SetSimulatePhysics (Variables|/Script/Engine.StaticMeshActor|GetStaticMeshComponent _returnvalue) false)
  (Transformation|AttachComponentToComponent (VehicleSound|GetRootComponent _returnvalue) (stale EventTeapotPickup AttachTo) "None" "KeepWorld" "KeepWorld" "KeepWorld" false))

(event Custom|CustomEvent_1
  ;[1 1 1] Several Zombies sketch
  (Actor|DestroyActor (stale _array_element)))

(event Custom|DestroyZombieonServer
  (Actor|DestroyActor (Variables|Default|GetDestroyActor)))

(event EventSetinInventory?
  (params (inInventory? :type Boolean))
  ;[1 1 1] Set functions
  (Variables|Default|SetinInventory? inInventory?))

(event EventTeapotPickup
  (params (AttachTo :type Scene%20Component%20Object%20Reference))
  ;[1 1 1] Regular pickup
  (if (Variables|Default|GetinInventory?)
    ;[1 1 1] MP test
    (CallFunction|MakeServerweapon)
    (bind _asteapot_player_controller (Utilities|Casting|CastToTeapot_PlayerController (Game|GetPlayerController 0)))
    (Utilities|Array|SetArrayElem (Variables|/Game/Teapot_Content/Blueprints/Teapot_PlayerController.Teapot_PlayerController_C|GetInventory _asteapot_player_controller) (Variables|Default|Getinventoryindex) 0)
    (Variables|Default|Setinventoryindex 10)
    (bind _outactors (Actor|GetAllActorsOfClass "/Game/Teapot_Content/Blueprints/Teapot_Inventory_Screen.Teapot_Inventory_Screen_C"))
    (Utilities|Array|RemoveItem (Variables|/Game/Teapot_Content/Blueprints/Teapot_Inventory_Screen.Teapot_Inventory_Screen_C|GetSpawnedActors (Utilities|Array|Get(acopy) _outactors)) self)
    (Actor|DestroyActor)
    (else
      (Physics|SetSimulatePhysics (Variables|Debug|GetStaticMeshComponent) false)
      (Transformation|AttachComponentToComponent (VehicleSound|GetRootComponent) AttachTo "None" "KeepWorld" "KeepWorld" "KeepWorld" false))))

(event EventTeapotDrop
  ;[1 1 1] Regular drop
  (if (not (Variables|Default|GetinInventory?))
    (Physics|SetSimulatePhysics (Variables|Debug|GetStaticMeshComponent) true)
    (Transformation|DetachFromActor "KeepRelative" "KeepRelative" "KeepRelative")))

(event EventSetinventoryindex
  (params (Inventoryindex :type Integer))
  ;[1 1 1] Set functions
  (Variables|Default|Setinventoryindex Inventoryindex))

(fn ConstructionScript)

(fn GetCanbreakdoor
  (return (Variables|WeaponProperties|GetCanbreakdoor)))

(fn GetDamage
  (return (Variables|Default|GetDamage)))

(fn GetinInventory?
  (return (Variables|Default|GetinInventory?)))

(fn GetisMelee
  (return (Variables|WeaponProperties|GetisMelee)))

(fn GetisSilent
  (return (Variables|WeaponProperties|GetisSilent)))

(fn GetisThrowable
  (return (Variables|WeaponProperties|GetisThrowable)))

(fn Weaponhit?
  (bind _index (Utilities|FlowControl|ForLoopwithBreak 1 (Variables|Default|GetDices))
    (:LoopBody
      (Utilities|Array|SetArrayElem (Variables|Default|GetHit) _index (>= (Math|Random|RandomInteger 6) (Variables|Default|GetHitchance)) true))
    (:Completed
      (return (Variables|Default|GetHit)))))