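; Base Blueprint for pickup weapons, providing pick-up and drop behavior plus weapon capability queries.
; TeapotPickup stops physics simulation on the static mesh and attaches the root component to the supplied component, keeping its world transform.
; TeapotDrop turns physics back on and detaches the actor using relative transform rules.
; Simple getters expose flags for door breaking, melee and throwable, with no logic here acting on them.
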(event EventBeginPlay)

(event EventTick
  (params (DeltaSeconds :type Float%20%28single-precision%29)))

(event EventTeapotPickup
  (params (AttachTo :type Scene%20Component%20Object%20Reference))
  (Physics|SetSimulatePhysics (Variables|Debug|GetStaticMeshComponent) false)
  (Transformation|AttachComponentToComponent (VehicleSound|GetRootComponent) AttachTo "None" "KeepWorld" "KeepWorld" "KeepWorld" false))

(event EventTeapotDrop
  (Physics|SetSimulatePhysics (Variables|Debug|GetStaticMeshComponent) true)
  (Transformation|DetachFromActor "KeepRelative" "KeepRelative" "KeepRelative"))

(fn ConstructionScript)

(fn GetCanbreakdoor
  (return (Variables|WeaponProperties|GetCanbreakdoor)))

(fn GetisMelee
  (return (Variables|WeaponProperties|GetisMelee)))

(fn GetisThrowable
  (return (Variables|WeaponProperties|GetisThrowable)))