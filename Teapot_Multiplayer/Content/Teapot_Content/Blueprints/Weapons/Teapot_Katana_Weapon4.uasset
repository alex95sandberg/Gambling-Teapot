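; A katana weapon actor that can be picked up, dropped and stored in the player's inventory.
; Pickup disables physics and attaches it to the given component; when taken from inventory, it also updates the player controller's slot and the inventory screen's spawned actors.
; Dropping detaches it and restores physics unless it is stored.
; Getters expose combat traits, and a hit check rolls several dice against a hit chance, returning per-die results.
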(event EventSetinInventory?
  (params (inInventory? :type Boolean))
  ;[1 1 1] Set functions
  (Variables|Default|SetinInventory? inInventory?))

(event EventTeapotPickup
  (params (AttachTo :type Scene%20Component%20Object%20Reference))
  ;[1 1 1] Regular pickup
  (Physics|SetSimulatePhysics (Variables|Debug|GetStaticMeshComponent) false)
  (Transformation|AttachComponentToComponent (VehicleSound|GetRootComponent) AttachTo "None" "KeepWorld" "KeepWorld" "KeepWorld" false)
  ;[1 1 1] Inventory management
  (if (Variables|Default|GetinInventory?)
    (Collision|SetCollisionEnabled (Variables|Debug|GetStaticMeshComponent) "QueryAndPhysics")
    (Variables|Default|SetinInventory? false)
    (bind _asteapot_player_controller (Utilities|Casting|CastToTeapot_PlayerController (Game|GetPlayerController 0)))
    (Utilities|Array|SetArrayElem (Variables|/Game/Teapot_Content/Blueprints/Teapot_PlayerController.Teapot_PlayerController_C|GetInventory _asteapot_player_controller) (Variables|Default|Getinventoryindex) 0)
    (Variables|Default|Setinventoryindex 10)
    (bind _outactors (Actor|GetAllActorsOfClass "/Game/Teapot_Content/Blueprints/Teapot_Inventory_Screen.Teapot_Inventory_Screen_C"))
    (bind _asteapot_inventory_screen (Utilities|Casting|CastToTeapot_Inventory_Screen (Utilities|Array|Get(acopy) _outactors)))
    (Utilities|Array|RemoveItem (Variables|/Game/Teapot_Content/Blueprints/Teapot_Inventory_Screen.Teapot_Inventory_Screen_C|GetSpawnedActors _asteapot_inventory_screen) self)))

(event EventTeapotDrop
  (if (not (Variables|Default|GetinInventory?))
    (Physics|SetSimulatePhysics (Variables|Debug|GetStaticMeshComponent) true)
    (Transformation|DetachFromActor "KeepRelative" "KeepRelative" "KeepRelative")))

(event EventSetinventoryindex
  (params (Inventoryindex :type Integer))
  ;[1 1 1] Set functions
  (Variables|Default|Setinventoryindex Inventoryindex))

(fn ConstructionScript)

(fn GetCanbreakdoor
  (return (Variables|WeaponProperties|GetCanbreakdoor)))

(fn GetDamage
  (return (Variables|Default|GetDamage)))

(fn GetinInventory?
  (return (Variables|Default|GetinInventory?)))

(fn GetisMelee
  (return (Variables|WeaponProperties|GetisMelee)))

(fn GetisSilent
  (return (Variables|WeaponProperties|GetisSilent)))

(fn GetisThrowable
  (return (Variables|WeaponProperties|GetisThrowable)))

(fn Weaponhit?
  (Utilities|FlowControl|ForLoopwithBreak 1 (Variables|Default|GetDices)
    (:LoopBody
      (Utilities|Array|AppendArray (Utilities|Array|MakeArray (>= (Math|Random|RandomInteger 5) (Variables|Default|GetHitchance))) (Variables|Default|GetHit)))
    (:Completed
      (return (Variables|Default|GetHit)))))