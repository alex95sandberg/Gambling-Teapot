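; Handgun weapon actor for the Teapot game that can be picked up, dropped and flagged as in inventory.
; Pickup stops physics simulation and attaches it to a given component; drop re-enables physics and detaches it.
; Getters expose damage, inventory state and traits such as melee, silent, throwable and door-breaking.
; Weaponhit? loops once per die, testing a random roll against Hitchance, and returns the Hit array.
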(event EventBeginPlay)

(event EventSetinInventory?
  (params (inInventory? :type Boolean))
  (Variables|Default|SetinInventory? inInventory?))

(event EventTick
  (params (DeltaSeconds :type Float%20%28single-precision%29)))

(event EventTeapotPickup
  (params (AttachTo :type Scene%20Component%20Object%20Reference))
  (bind _staticmeshcomponent (Variables|Debug|GetStaticMeshComponent))
  (Physics|SetSimulatePhysics _staticmeshcomponent false)
  (Collision|SetCollisionEnabled _staticmeshcomponent "QueryAndPhysics")
  (Transformation|AttachComponentToComponent (VehicleSound|GetRootComponent) AttachTo "None" "KeepWorld" "KeepWorld" "KeepWorld" false))

(event EventTeapotDrop
  (Physics|SetSimulatePhysics (Variables|Debug|GetStaticMeshComponent) true)
  (Transformation|DetachFromActor "KeepRelative" "KeepRelative" "KeepRelative"))

(fn ConstructionScript)

(fn GetCanbreakdoor
  (return (Variables|WeaponProperties|GetCanbreakdoor)))

(fn GetDamage
  (return (Variables|Default|GetDamage)))

(fn GetinInventory?
  (return (Variables|Default|GetinInventory?)))

(fn GetisMelee
  (return (Variables|WeaponProperties|GetisMelee)))

(fn GetisSilent
  (return (Variables|WeaponProperties|GetisSilent)))

(fn GetisThrowable
  (return (Variables|WeaponProperties|GetisThrowable)))

(fn Weaponhit?
  (Utilities|FlowControl|ForLoopwithBreak 1 (Variables|Default|GetDices)
    (:LoopBody
      (Utilities|Array|AppendArray (Utilities|Array|MakeArray (>= (Math|Random|RandomInteger 5) (Variables|Default|GetHitchance))) (Variables|Default|GetHit)))
    (:Completed
      (return (Variables|Default|GetHit)))))