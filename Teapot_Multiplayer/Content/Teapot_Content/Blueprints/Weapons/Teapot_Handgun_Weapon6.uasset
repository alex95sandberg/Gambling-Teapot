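; Handgun weapon for a turn-based, tile-based VR zombie game, grabbed by motion controllers or taken from inventory by spawning an attached replacement.
; On the player's turn with actions left, melee overlap targets a same-tile zombie, while shooting line-traces from the hand to a tile.
; HitTheZombie spends an action, rolls dice against Hitchance, flashes a green or red cube, and destroys the zombie on any hit.
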(event OnComponentBeginOverlap(StaticMeshComponent)
  (params (OverlappedComponent :type Primitive%20Component%20Object%20Reference) (OtherActor :type Actor%20Object%20Reference) (OtherComp :type Primitive%20Component%20Object%20Reference) (OtherBodyIndex :type Integer) (bFromSweep :type Boolean) (SweepResult :type Hit%20Result%20Structure%20%28by%20ref%29))
  ;[1 1 1] Can only hit one Zombie
  (bind _asteapot_vrpawn (Utilities|Casting|CastToTeapot_VRPawn (Game|Player|GetPlayerPawn 0)))
  (bind _asteapot_zombie (Utilities|Casting|CastToTeapot_Zombie OtherActor))
  (if (== (Variables|/Game/Teapot_Content/Blueprints/Teapot_Zombie.Teapot_Zombie_C|GetCurrentTile _asteapot_zombie) (Variables|/Game/Teapot_Content/Blueprints/Teapot_PlayerBody.Teapot_PlayerBody_C|GetCurrentTile (Variables|/Game/Teapot_Content/Blueprints/Teapot_VRPawn.Teapot_VRPawn_C|GetPlayerBody _asteapot_vrpawn)))
    (bind _asteapot_game_state (Utilities|Casting|CastToTeapot_GameState (Game|GetGameState)))
    (bind _ismyturn (Default|IsMyTurn _asteapot_game_state))
    (if (Math|Boolean|ANDBoolean (>= (Variables|/Game/Teapot_Content/Blueprints/Teapot_GameState.Teapot_GameState_C|GetRemainingActions _asteapot_game_state) 1) _ismyturn (Variables|WeaponProperties|GetisMelee) (not (Variables|Default|GetinInventory?)))
      (Variables|Default|SetDestroyActor _asteapot_zombie)
      (Utilities|HittheZombie _asteapot_game_state))))

(event Custom|Make%20Serverweapon
  (bind _self self)
  ;[1 1 1] MP test
  (bind _returnvalue (Game|SpawnActorfromClass "Teapot_Handgun_Weapon6_C" (Math|Transform|MakeTransform (Transformation|GetActorLocation _self) (Transformation|GetActorRotation _self)) "AlwaysSpawn" 0 0))
  (Physics|SetSimulatePhysics (Variables|/Script/Engine.StaticMeshActor|GetStaticMeshComponent _returnvalue) false)
  (Transformation|AttachComponentToComponent (VehicleSound|GetRootComponent _returnvalue) (stale EventTeapotPickup AttachTo) "None" "KeepWorld" "KeepWorld" "KeepWorld" false)
  (bind _asteapot_motion_controller (Utilities|Casting|CastToTeapot_MotionController (Components|GetOwner (stale EventTeapotPickup AttachTo))))
  (Variables|/Game/Teapot_Content/Blueprints/Teapot_MotionController.Teapot_MotionController_C|SetAttachedActor _asteapot_motion_controller _returnvalue))

(event Custom|CustomEvent_1
  ;[1 1 1] Several Zombies sketch
  (Actor|DestroyActor (stale _array_element)))

(event Custom|DestroyZombieonServer
  (if (Variables|Default|GetKill?)
    (Actor|DestroyActor (Variables|Default|GetDestroyActor)))
  (Actor|DestroyActor (Variables|Default|GetIndicatorActor)))

(event Custom|ChangeMaterialServer
  (bind _indicatoractor (Variables|Default|GetIndicatorActor))
  (bind _staticmeshcomponent (Variables|/Script/Engine.StaticMeshActor|GetStaticMeshComponent _indicatoractor))
  (if (Variables|Default|GetKill?)
    (Rendering|Material|SetMaterial _staticmeshcomponent 0 "/Game/Teapot_Content/Materials/Teapot_Green.Teapot_Green")
    (else
      (Rendering|Material|SetMaterial _staticmeshcomponent 0 "/Game/Teapot_Content/Materials/Teapot_Red.Teapot_Red"))))

(event EventShoot!
  (bind _asteapot_game_state (Utilities|Casting|CastToTeapot_GameState (Game|GetGameState)))
  (bind _ismyturn (Default|IsMyTurn _asteapot_game_state))
  (if (Math|Boolean|ANDBoolean (>= (Variables|/Game/Teapot_Content/Blueprints/Teapot_GameState.Teapot_GameState_C|GetRemainingActions _asteapot_game_state) 1) _ismyturn (not (Variables|WeaponProperties|GetisMelee)) (not (Variables|Default|GetinInventory?)))
    (bind _asteapot_motion_controller (Utilities|Casting|CastToTeapot_MotionController (Actor|GetAttachParentActor)))
    (bind _outhit (Collision|LineTraceByChannel (Transformation|GetWorldLocation (Variables|/Game/Teapot_Content/Blueprints/Teapot_MotionController.Teapot_MotionController_C|GetHandMesh _asteapot_motion_controller)) (+ (Transformation|GetWorldLocation (Variables|/Game/Teapot_Content/Blueprints/Teapot_MotionController.Teapot_MotionController_C|GetHandMesh _asteapot_motion_controller)) (* (Math|Vector|GetForwardVector (Transformation|GetWorldRotation (Variables|/Game/Teapot_Content/Blueprints/Teapot_MotionController.Teapot_MotionController_C|GetHandMesh _asteapot_motion_controller))) 1e+03)) "TraceTypeQuery1" false 0 "ForDuration" true "(R=1.000000,G=0.000000,B=0.000000,A=1.000000)" "(R=0.000000,G=1.000000,B=0.000000,A=1.000000)" 2.0))
    (bind _asteapot_tile (Utilities|Casting|CastToTeapot_Tile (.hitactor _outhit)))
    (bind _outactors (Actor|GetAllActorsOfClass "/Game/Teapot_Content/Blueprints/Teapot_Zombie.Teapot_Zombie_C"))
    (bind _array_element (Utilities|Array|ForEachLoopwithBreak _outactors :!label _label)
      (:LoopBody
        (bind _asteapot_zombie (Utilities|Casting|CastToTeapot_Zombie _array_element))
        (if (== (Variables|/Game/Teapot_Content/Blueprints/Teapot_Zombie.Teapot_Zombie_C|GetCurrentTile _asteapot_zombie) _asteapot_tile)
          (Variables|Default|SetRangeZombieFound true)
          (Variables|Default|SetDestroyActor _asteapot_zombie)
          (goto _label Break)))
      (:Completed
        (if (Variables|Default|GetRangeZombieFound)
          (Variables|Default|SetRangeZombieFound false)
          (Utilities|HittheZombie _asteapot_game_state))))))

(event EventSetinInventory?
  (params (inInventory? :type Boolean))
  ;[1 1 1] Set functions
  (Variables|Default|SetinInventory? inInventory?))

(event EventTeapotPickup
  (params (AttachTo :type Scene%20Component%20Object%20Reference))
  ;[1 1 1] Regular pickup
  (if (Variables|Default|GetinInventory?)
    ;[1 1 1] MP test
    (CallFunction|MakeServerweapon)
    (bind _asteapot_player_controller (Utilities|Casting|CastToTeapot_PlayerController (Game|GetPlayerController 0)))
    (Utilities|Array|SetArrayElem (Variables|/Game/Teapot_Content/Blueprints/Teapot_PlayerController.Teapot_PlayerController_C|GetInventory _asteapot_player_controller) (Variables|Default|Getinventoryindex) 0)
    (Variables|Default|Setinventoryindex 10)
    (bind _outactors (Actor|GetAllActorsOfClass "/Game/Teapot_Content/Blueprints/Teapot_Inventory_Screen.Teapot_Inventory_Screen_C"))
    (Utilities|Array|RemoveItem (Variables|/Game/Teapot_Content/Blueprints/Teapot_Inventory_Screen.Teapot_Inventory_Screen_C|GetSpawnedActors (Utilities|Array|Get(acopy) _outactors)) self)
    (Actor|DestroyActor)
    (else
      (Physics|SetSimulatePhysics (Variables|Debug|GetStaticMeshComponent) false)
      (Transformation|AttachComponentToComponent (VehicleSound|GetRootComponent) AttachTo "None" "KeepWorld" "KeepWorld" "KeepWorld" false))))

(event EventTeapotDrop
  ;[1 1 1] Regular drop
  (if (not (Variables|Default|GetinInventory?))
    (Physics|SetSimulatePhysics (Variables|Debug|GetStaticMeshComponent) true)
    (Transformation|DetachFromActor "KeepRelative" "KeepRelative" "KeepRelative")))

(event EventSetinventoryindex
  (params (Inventoryindex :type Integer))
  ;[1 1 1] Set functions
  (Variables|Default|Setinventoryindex Inventoryindex))

(fn ConstructionScript)

(fn GetCanbreakdoor
  (return (Variables|WeaponProperties|GetCanbreakdoor)))

(fn GetDamage
  (return (Variables|Default|GetDamage)))

(fn GetinInventory?
  (return (Variables|Default|GetinInventory?)))

(fn GetisMelee
  (return (Variables|WeaponProperties|GetisMelee)))

(fn GetisSilent
  (return (Variables|WeaponProperties|GetisSilent)))

(fn GetisThrowable
  (return (Variables|WeaponProperties|GetisThrowable)))

(fn Weaponhit?
  (bind _index (Utilities|FlowControl|ForLoopwithBreak 1 (Variables|Default|GetDices))
    (:LoopBody
      (Utilities|Array|SetArrayElem (Variables|Default|GetHit) _index (>= (Math|Random|RandomInteger 6) (Variables|Default|GetHitchance)) true))
    (:Completed
      (return (Variables|Default|GetHit)))))