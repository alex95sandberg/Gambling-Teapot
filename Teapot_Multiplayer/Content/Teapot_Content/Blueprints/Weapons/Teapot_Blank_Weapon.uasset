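; Blank weapon Blueprint for Teapot, apparently a base or template for weapons with dice-based hit checks.
; Getter functions expose damage and flags for door breaking, melee, silent and throwable, while the inventory check always returns false.
; Weaponhit? rolls a random integer per die, compares it to Hitchance in an array append step, and returns the Hit array.
; The event graph and construction script are empty.
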(event EventBeginPlay)

(event EventTick
  (params (DeltaSeconds :type Float%20%28single-precision%29)))

(fn ConstructionScript)

(fn GetCanbreakdoor
  (return (Variables|WeaponProperties|GetCanbreakdoor)))

(fn GetDamage
  (return (Variables|Default|GetDamage)))

(fn GetinInventory?
  (return false))

(fn GetisMelee
  (return (Variables|WeaponProperties|GetisMelee)))

(fn GetisSilent
  (return (Variables|WeaponProperties|GetisSilent)))

(fn GetisThrowable
  (return (Variables|WeaponProperties|GetisThrowable)))

(fn Weaponhit?
  (Utilities|FlowControl|ForLoopwithBreak 1 (Variables|Default|GetDices)
    (:LoopBody
      (Utilities|Array|AppendArray (Utilities|Array|MakeArray (>= (Math|Random|RandomInteger 5) (Variables|Default|GetHitchance))) (Variables|Default|GetHit)))
    (:Completed
      (return (Variables|Default|GetHit)))))