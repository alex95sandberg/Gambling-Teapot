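; Weapon actor for a turn-based, tile-based VR zombie game, with melee, ranged, flashlight toggle, and pickup, drop and inventory handling.
; Melee triggers on mesh overlap with a same-tile zombie, while ranged line-traces from the hand to a tile and finds a zombie there.
; Both check turn, actions and inventory state, then call HitTheZombie, which rolls dice, briefly shows a green or red indicator cube and destroys the zombie on success.
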(event OnComponentBeginOverlap(StaticMeshComponent)
  (params (OverlappedComponent :type Primitive%20Component%20Object%20Reference) (OtherActor :type Actor%20Object%20Reference) (OtherComp :type Primitive%20Component%20Object%20Reference) (OtherBodyIndex :type Integer) (bFromSweep :type Boolean) (SweepResult :type Hit%20Result%20Structure%20%28by%20ref%29))
  (bind _staticmeshcomponent (Variables|Debug|GetStaticMeshComponent))
  ;[1 1 1] Melee interaction with Zombie
  (bind _asteapot_zombie_standard (Utilities|Casting|CastToTeapot_Zombie_Standard OtherActor))
  (bind _asteapot_vrpawn (Utilities|Casting|CastToTeapot_VRPawn (Actor|GetAttachParentActor (Actor|GetAttachParentActor self))))
  (if (== (Variables|/Game/Teapot_Content/Blueprints/Teapot_PlayerBody.Teapot_PlayerBody_C|GetCurrentTile (Variables|/Game/Teapot_Content/Blueprints/Teapot_VRPawn.Teapot_VRPawn_C|GetPlayerBody _asteapot_vrpawn)) (Variables|/Game/Teapot_Content/Blueprints/Teapot_Zombie_Standard.Teapot_Zombie_Standard_C|GetCurrentTile _asteapot_zombie_standard))
    (bind _asteapot_player_controller (Utilities|Casting|CastToTeapot_PlayerController (Pawn|GetController _asteapot_vrpawn)))
    (bind _asteapot_game_mode (Utilities|Casting|CastToTeapot_GameMode (Game|GetGameMode)))
    (bind _asteapot_player_state (Utilities|Casting|CastToTeapot_PlayerState (Variables|/Script/Engine.Controller|GetPlayerState _asteapot_player_controller)))
    (if (Math|Boolean|ANDBoolean (>= (Variables|/Game/Teapot_Content/Blueprints/Teapot_PlayerState.Teapot_PlayerState_C|GetRemainingActions _asteapot_player_state) 1) (Variables|WeaponProperties|GetisMelee) (not (Variables|Default|GetinInventory?)) (== (Variables|/Game/Teapot_Content/Blueprints/Teapot_GameMode.Teapot_GameMode_C|GetTurnIndex _asteapot_game_mode) (Variables|/Game/Teapot_Content/Blueprints/Teapot_PlayerController.Teapot_PlayerController_C|GetPlayerIndex _asteapot_player_controller)))
      (Default|ReduceActionsClient _asteapot_vrpawn 1)
      (Variables|Default|SetDestroyActor _asteapot_zombie_standard)
      (Variables|/Script/Engine.PrimitiveComponent|SetbGenerateOverlapEvents _staticmeshcomponent false)
      (Utilities|HittheZombie
        (:Exec
          (Variables|/Script/Engine.PrimitiveComponent|SetbGenerateOverlapEvents _staticmeshcomponent true))))))

(event Custom|Make%20Serverweapon
  (params (Attachedto :type Scene%20Component%20Object%20Reference))
  (bind _self self)
  ;[1 1 1] MP test, not currently in use
  (bind _returnvalue (Game|SpawnActorfromClass "/Game/Teapot_Content/Blueprints/Weapons/Teapot_Base_Weapon.Teapot_Base_Weapon_C" (Math|Transform|MakeTransform (Transformation|GetActorLocation _self) (Transformation|GetActorRotation _self)) "AlwaysSpawn" 0 0))
  (Physics|SetSimulatePhysics (Variables|/Script/Engine.StaticMeshActor|GetStaticMeshComponent _returnvalue) false)
  (Transformation|AttachComponentToComponent (VehicleSound|GetRootComponent _returnvalue) Attachedto "None" "KeepWorld" "KeepWorld" "KeepWorld" false)
  (bind _asteapot_motion_controller (Utilities|Casting|CastToTeapot_MotionController (Components|GetOwner Attachedto)))
  (Variables|/Game/Teapot_Content/Blueprints/Teapot_MotionController.Teapot_MotionController_C|SetAttachedActor _asteapot_motion_controller _returnvalue))

(event Custom|CustomEvent_1
  ;[1 1 1] Several Zombies sketch
  (Actor|DestroyActor (stale _array_element)))

(event Custom|DestroyZombieonServer
  ;[1 1 1] Server events
  (if (Variables|Default|GetKill?)
    (Actor|DestroyActor (Variables|Default|GetDestroyActor)))
  (Actor|DestroyActor (Variables|Default|GetIndicatorActor)))

(event Custom|ChangeMaterialServer
  (bind _indicatoractor (Variables|Default|GetIndicatorActor))
  (bind _staticmeshcomponent (Variables|/Script/Engine.StaticMeshActor|GetStaticMeshComponent _indicatoractor))
  ;[1 1 1] Server events
  (if (Variables|Default|GetKill?)
    (Rendering|Material|SetMaterial _staticmeshcomponent 0 "/Game/Teapot_Content/Materials/Teapot_Green.Teapot_Green")
    (else
      (Rendering|Material|SetMaterial _staticmeshcomponent 0 "/Game/Teapot_Content/Materials/Teapot_Red.Teapot_Red"))))

(event EventShoot!
  (params (WhoPawn? :type Teapot%20VR%20Pawn%20Object%20Reference))
  ;[1 1 1] Ranged interaction with Zombie
  (if (Variables|Default|GetFlashlight?)
    (bind _asteapot_flashlight_weapon_6 (Utilities|Casting|CastToTeapot_Flashlight_Weapon6 self))
    (Rendering|SetVisibility (Variables|/Game/Teapot_Content/Blueprints/Weapons/Teapot_Flashlight_Weapon6.Teapot_Flashlight_Weapon6_C|GetSpotLight _asteapot_flashlight_weapon_6) (not (Variables|/Script/Engine.SceneComponent|GetbVisible (Variables|/Game/Teapot_Content/Blueprints/Weapons/Teapot_Flashlight_Weapon6.Teapot_Flashlight_Weapon6_C|GetSpotLight _asteapot_flashlight_weapon_6))) false)
    (else
      (bind _asteapot_player_controller (Utilities|Casting|CastToTeapot_PlayerController (Pawn|GetController WhoPawn?)))
      (bind _asteapot_vrpawn (Utilities|Casting|CastToTeapot_VRPawn (Pawn|GetControlledPawn _asteapot_player_controller)))
      (bind _asteapot_game_mode (Utilities|Casting|CastToTeapot_GameMode (Game|GetGameMode)))
      (bind _asteapot_player_state (Utilities|Casting|CastToTeapot_PlayerState (Variables|/Script/Engine.Controller|GetPlayerState _asteapot_player_controller)))
      (if (Math|Boolean|ANDBoolean (>= (Variables|/Game/Teapot_Content/Blueprints/Teapot_PlayerState.Teapot_PlayerState_C|GetRemainingActions _asteapot_player_state) 1) (not (Variables|WeaponProperties|GetisMelee)) (not (Variables|Default|GetinInventory?)) (== (Variables|/Game/Teapot_Content/Blueprints/Teapot_GameMode.Teapot_GameMode_C|GetTurnIndex _asteapot_game_mode) (Variables|/Game/Teapot_Content/Blueprints/Teapot_PlayerController.Teapot_PlayerController_C|GetPlayerIndex _asteapot_player_controller)))
        (bind _asteapot_motion_controller (Utilities|Casting|CastToTeapot_MotionController (Actor|GetAttachParentActor)))
        (bind _outhit (Collision|LineTraceByChannel (Transformation|GetWorldLocation (Variables|/Game/Teapot_Content/Blueprints/Teapot_MotionController.Teapot_MotionController_C|GetHandMesh _asteapot_motion_controller)) (+ (Transformation|GetWorldLocation (Variables|/Game/Teapot_Content/Blueprints/Teapot_MotionController.Teapot_MotionController_C|GetHandMesh _asteapot_motion_controller)) (* (Math|Vector|GetForwardVector (Transformation|GetWorldRotation (Variables|/Game/Teapot_Content/Blueprints/Teapot_MotionController.Teapot_MotionController_C|GetHandMesh _asteapot_motion_controller))) 1e+03)) "TraceTypeQuery1" false 0 "ForDuration" true "(R=1.000000,G=0.000000,B=0.000000,A=1.000000)" "(R=0.000000,G=1.000000,B=0.000000,A=1.000000)" 2.0))
        (bind _asteapot_tile (Utilities|Casting|CastToTeapot_Tile (.hitactor _outhit)))
        (bind _outactors (Actor|GetAllActorsOfClass "/Game/Teapot_Content/Blueprints/Teapot_Zombie_Standard.Teapot_Zombie_Standard_C"))
        (bind _array_element (Utilities|Array|ForEachLoopwithBreak _outactors :!label _label)
          (:LoopBody
            (bind _asteapot_zombie_standard (Utilities|Casting|CastToTeapot_Zombie_Standard _array_element))
            (if (== (Variables|/Game/Teapot_Content/Blueprints/Teapot_Zombie_Standard.Teapot_Zombie_Standard_C|GetCurrentTile _asteapot_zombie_standard) _asteapot_tile)
              (Variables|Default|SetRangeZombieFound true)
              (Variables|Default|SetDestroyActor _asteapot_zombie_standard)
              (goto _label Break)))
          (:Completed
            (if (Variables|Default|GetRangeZombieFound)
              (Variables|Default|SetRangeZombieFound false)
              (Default|ReduceActionsClient _asteapot_vrpawn)
              (Utilities|HittheZombie))))))))

(event EventSetinInventory?
  (params (inInventory? :type Boolean))
  ;[1 1 1] Set functions
  (Variables|Default|SetinInventory? inInventory?))

(event EventTeapotPickup
  (params (AttachTo :type Scene%20Component%20Object%20Reference) (PlayerIndex :type Integer))
  ;[1 1 1] On pickup
  (Physics|SetSimulatePhysics (Variables|Debug|GetStaticMeshComponent) false)
  (Transformation|AttachComponentToComponent (VehicleSound|GetRootComponent) AttachTo "None" "KeepWorld" "KeepWorld" "KeepWorld" false)
  (if (Variables|Default|GetinInventory?)
    (Variables|Default|SetinInventory? false)
    (Collision|SetCollisionEnabled (Variables|Debug|GetStaticMeshComponent) "QueryAndPhysics")
    (bind _asteapot_player_controller (Utilities|Casting|CastToTeapot_PlayerController (Game|GetPlayerController 0)))
    (Utilities|Array|SetArrayElem (Variables|/Game/Teapot_Content/Blueprints/Teapot_PlayerController.Teapot_PlayerController_C|GetInventory _asteapot_player_controller) (Variables|Default|Getinventoryindex) 0)
    (Variables|Default|Setinventoryindex 10)
    (bind _outactors (Actor|GetAllActorsOfClass "/Game/Teapot_Content/Blueprints/Teapot_Inventory_Screen.Teapot_Inventory_Screen_C"))
    (Utilities|Array|RemoveItem (Variables|/Game/Teapot_Content/Blueprints/Teapot_Inventory_Screen.Teapot_Inventory_Screen_C|GetSpawnedActors (Utilities|Array|Get(acopy) _outactors)) self)))

(event EventTeapotDrop
  ;[1 1 1] On drop
  (if (not (Variables|Default|GetinInventory?))
    (Physics|SetSimulatePhysics (Variables|Debug|GetStaticMeshComponent) true)
    (Transformation|DetachFromActor "KeepRelative" "KeepRelative" "KeepRelative")))

(event EventSetinventoryindex
  (params (Inventoryindex :type Integer))
  ;[1 1 1] Set functions
  (Variables|Default|Setinventoryindex Inventoryindex))

(fn ConstructionScript)

(fn GetCanbreakdoor
  (return (Variables|WeaponProperties|GetCanbreakdoor)))

(fn GetDamage
  (return (Variables|Default|GetDamage)))

(fn GetinInventory?
  (return (Variables|Default|GetinInventory?)))

(fn GetisMelee
  (return (Variables|WeaponProperties|GetisMelee)))

(fn GetisSilent
  (return (Variables|WeaponProperties|GetisSilent)))

(fn GetisThrowable
  (return (Variables|WeaponProperties|GetisThrowable)))

(fn Weaponhit?
  (bind _index (Utilities|FlowControl|ForLoopwithBreak 1 (Variables|Default|GetDices))
    (:LoopBody
      (Utilities|Array|SetArrayElem (Variables|Default|GetHit) _index (>= (Math|Random|RandomInteger 6) (Variables|Default|GetHitchance)) true))
    (:Completed
      (return (Variables|Default|GetHit)))))