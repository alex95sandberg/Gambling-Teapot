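; Teapot_PlayerState is the player state for a turn-based VR game on tiles, handling action points, turn checks and tile noise.
; ReduceRemainingActions subtracts from the remaining actions and pushes the count to the controlled VR pawn's actions text.
; IsMyTurn compares the owning controller's player index with the game mode's turn index.
; UpdateNoise moves one noise point from the previous tile to the new one and prints a debug message.
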(event Custom|UpdateNoise
  (params (PreviousTile :type Teapot%20Tile%20Object%20Reference) (NewTile :type Teapot%20Tile%20Object%20Reference))
  ;[1 1 1] Update Noise
  (Utilities|IsValid PreviousTile
    (:Is%20Valid
      (bind _result (Math|Integer|DecrementInt (Variables|/Game/Teapot_Content/Blueprints/Teapot_Tile.Teapot_Tile_C|GetNoise PreviousTile))
        (:%20%20
          (Variables|/Game/Teapot_Content/Blueprints/Teapot_Tile.Teapot_Tile_C|SetNoise PreviousTile _result))))
    (:Is%20Not%20Valid
      _))
  (bind _result_2 (Math|Integer|IncrementInt (Variables|/Game/Teapot_Content/Blueprints/Teapot_Tile.Teapot_Tile_C|GetNoise NewTile))
    (:%20%20
      (Variables|/Game/Teapot_Content/Blueprints/Teapot_Tile.Teapot_Tile_C|SetNoise NewTile _result_2)
      (Development|PrintString (Utilities|String|Append "Updated noise for Player" "") true true "(R=0.000000,G=0.660000,B=1.000000,A=1.000000)" 5.0))))

(event EventBeginPlay)

(event EventTick
  (params (DeltaSeconds :type Float%20%28single-precision%29)))

(fn ConstructionScript)

(fn ReduceRemainingActions
  (params (Amount :type Integer))
  (bind _output_get (Variables|Default|SetRemainingActions (- (Variables|Default|GetRemainingActions) Amount)))
  (bind _asplayer_controller (Utilities|Casting|CastToPlayerController (Components|GetOwner)))
  (bind _asteapot_vrpawn (Utilities|Casting|CastToTeapot_VRPawn (Pawn|GetControlledPawn _asplayer_controller)))
  (Default|UpdateActionsText _asteapot_vrpawn _output_get))

(fn IsMyTurn?
  (bind _asteapot_player_controller (Utilities|Casting|CastToTeapot_PlayerController (Components|GetOwner))
    (:then
      (bind _asteapot_game_mode (Utilities|Casting|CastToTeapot_GameMode (Game|GetGameMode))
        (:then
          (return (== (Variables|/Game/Teapot_Content/Blueprints/Teapot_PlayerController.Teapot_PlayerController_C|GetPlayerIndex _asteapot_player_controller) (Variables|/Game/Teapot_Content/Blueprints/Teapot_GameMode.Teapot_GameMode_C|GetTurnIndex _asteapot_game_mode))))
        (:CastFailed
          _)))
    (:CastFailed
      (Development|PrintString "Debug: 
Cast Failed in IsMyTurn?" true true "(R=0.000000,G=0.660000,B=1.000000,A=1.000000)" 1e+01)))
  (return false))