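; World tile for a turn-based board game that registers player moves on overlap and mirrors them on a linked board tile.
; Moves from an existing tile require the player's turn, a connection and enough GameState actions, then charge the departed tile's cost.
; Entry updates noise and spotlights, then teleports the player's board pawn, spawned as needed, via MovePawnOnServer.
; Construction back-links the BoardTile; older nav-area movement code remains disconnected.
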(event Custom|IncrementNoise
  (bind _result (Math|Integer|IncrementInt (Variables|Default|GetNoise))
    (:%20%20
      (Variables|Default|SetNoise _result))))

(event Custom|MovePawnOnServer
  (params (BoardPawn :type Actor%20Object%20Reference))
  ;[1 1 1] Move to boardpawn on the server
  (Transformation|Teleport BoardPawn (+ (.Location (Math|Transform|BreakTransform (Transformation|GetActorTransform (Variables|Default|GetBoardTile)))) "0, 0,20.000000") "0, 0, 0"))

(event Custom|DecrementNoise
  (params (PreviousTile :type Teapot%20Tile%20Object%20Reference))
  (bind _result (Math|Integer|DecrementInt (Variables|Teapot_Tile_C|GetNoise PreviousTile))
    (:%20%20
      (Variables|Teapot_Tile_C|SetNoise PreviousTile _result))))

(event Collision|EventActorBeginOverlap
  (params (OtherActor :type Actor%20Object%20Reference))
  (bind _asteapot_game_state (Utilities|Casting|CastToTeapot_GameState (Game|GetGameState)))
  (bind _asteapot_player_body (Utilities|Casting|CastToTeapot_PlayerBody OtherActor))
  (bind _asteapot_tile (Utilities|Casting|CastToTeapot_Tile (Variables|/Game/Teapot_Content/Blueprints/Teapot_PlayerBody.Teapot_PlayerBody_C|GetCurrentTile _asteapot_player_body))
    (:then
      (bind _ispermitted (CallFunction|IsMovePermitted _asteapot_player_body _asteapot_tile))
      (if _ispermitted
        (CallFunction|DecrementNoise _asteapot_tile)
        (Default|ReduceRemainingActions _asteapot_game_state (Variables|Teapot_Tile_C|GetActionCost _asteapot_tile))
        (Rendering|SetVisibility (Variables|Teapot_Tile_C|GetSpotLight _asteapot_tile) true false)
        (Variables|/Game/Teapot_Content/Blueprints/Teapot_PlayerBody.Teapot_PlayerBody_C|SetCurrentTile _asteapot_player_body self :!label _label)
        (CallFunction|IncrementNoise)
        (Rendering|SetVisibility (Variables|Default|GetSpotLight) false false)
        (bind _boardpawn (CallFunction|MoveBoardPawn _asteapot_player_body))
        (CallFunction|MovePawnonServer _boardpawn)))
    (:CastFailed
      (goto _label))))

(fn ConstructionScript
  (bind _asteapot_board_tile (Utilities|Casting|CastToTeapot_BoardTile (Variables|Default|GetBoardTile)))
  (Variables|/Game/Teapot_Content/Blueprints/Teapot_BoardTile.Teapot_BoardTile_C|SetWorldTile _asteapot_board_tile self))

(fn MoveBoardPawn
  (params (PlayerBody :type Teapot%20Player%20Body%20Object%20Reference))
  (if (== (Variables|/Game/Teapot_Content/Blueprints/Teapot_PlayerBody.Teapot_PlayerBody_C|GetBoardPawn PlayerBody) 0)
    (bind _returnvalue (Game|SpawnActorfromClass "/Game/Teapot_Content/Blueprints/Teapot_PlayPawn.Teapot_PlayPawn_C" (Math|Transform|MakeTransform "0, 0, 0") "Undefined" 0 0))
    (Variables|/Game/Teapot_Content/Blueprints/Teapot_PlayerBody.Teapot_PlayerBody_C|SetBoardPawn PlayerBody _returnvalue)
    (bind _asteapot_player_controller (Utilities|Casting|CastToTeapot_PlayerController (Game|GetPlayerController 0)))
    (Variables|/Game/Teapot_Content/Blueprints/Teapot_PlayPawn.Teapot_PlayPawn_C|SetPlayerIndex _returnvalue (Variables|/Game/Teapot_Content/Blueprints/Teapot_PlayerController.Teapot_PlayerController_C|GetPlayerIndex _asteapot_player_controller)))
  (return (Variables|/Game/Teapot_Content/Blueprints/Teapot_PlayerBody.Teapot_PlayerBody_C|GetBoardPawn PlayerBody)))

(fn IsMovePermitted
  (params (PlayerBody :type Teapot%20Player%20Body%20Object%20Reference) (CurrentTile :type Teapot%20Tile%20Object%20Reference))
  (bind _self self)
  (bind _asteapot_game_state (Utilities|Casting|CastToTeapot_GameState (Game|GetGameState)))
  (bind _ismyturn (Default|IsMyTurn _asteapot_game_state))
  (return (Math|Boolean|ANDBoolean _ismyturn (Utilities|Array|ContainsItem (Variables|Teapot_Tile_C|GetConnectedTiles CurrentTile) _self) (!= CurrentTile _self) (<= (Variables|Teapot_Tile_C|GetActionCost CurrentTile) (Variables|/Game/Teapot_Content/Blueprints/Teapot_GameState.Teapot_GameState_C|GetRemainingActions _asteapot_game_state)))))