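; Game mode for a multiplayer, turn-based Teapot VR game that spawns players and tracks whose turn it is.
; On PostLogin in a particular game-instance state, the server gathers PlayerStarts, registers and indexes the controller, and possesses a new pawn at the next start.
; It also spawns a Teapot_PlayPawn per player and links it to the VR pawn.
; NextTurn cycles through registered controllers and copies the turn index to the game state.
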(event Custom|RunOnServerSpawnPlayer
  (params (PlayerController :type Player%20Controller%20Object%20Reference))
  (bind _returnvalue (Pawn|GetControlledPawn PlayerController))
  ;[1 1 1] PlayerIndex stuff
  (bind _asteapot_player_controller (Utilities|Casting|CastToTeapot_PlayerController PlayerController))
  (bind _returnvalue_2 (Utilities|Array|Add (Variables|Default|GetPlayerControllers) _asteapot_player_controller))
  (Variables|/Game/Teapot_Content/Blueprints/Teapot_PlayerController.Teapot_PlayerController_C|SetPlayerIndex _asteapot_player_controller _returnvalue_2)
  (Utilities|IsValid _returnvalue
    (:Is%20Valid
      (Actor|DestroyActor _returnvalue)
      (Development|PrintString "Destroyed Actor"))
    (:Is%20Not%20Valid
      _))
  (bind _returnvalue_3 (Game|SpawnActorfromClass (Variables|Default|GetPlayerPawn) (Transformation|GetActorTransform (Utilities|Array|Get(acopy) (Variables|Default|GetPlayerStartPoints) (Variables|Default|GetPlayerStartIndex))) "AlwaysSpawn" PlayerController 0))
  (bind _aspawn (Utilities|Casting|CastToPawn _returnvalue_3))
  (Pawn|Possess PlayerController _aspawn)
  (Variables|Default|SetPlayerStartIndex (+ (Variables|Default|GetPlayerStartIndex) 1))
  (bind _returnvalue_4 (Game|SpawnActorfromClass "/Game/Teapot_Content/Blueprints/Teapot_PlayPawn.Teapot_PlayPawn_C" (Math|Conversions|ToTransform(Vector) "0.000000, 0,140.000000") "Undefined" PlayerController 0))
  (bind _asteapot_vrpawn (Utilities|Casting|CastToTeapot_VRPawn _aspawn))
  (Variables|/Game/Teapot_Content/Blueprints/Teapot_VRPawn.Teapot_VRPawn_C|SetPlayPawn _asteapot_vrpawn _returnvalue_4))

(event EventBeginPlay)

(event EventTick
  (params (DeltaSeconds :type Float%20%28single-precision%29)))

(event EventPostLogin
  (params (NewPlayer :type Player%20Controller%20Object%20Reference))
  (Development|PrintString "OnPostLogin")
  (bind _asteapot_game_instance (Utilities|Casting|CastToTeapot_GameInstance (Game|GetGameInstance)))
  (bind _currentstate (Default|GetCurrentState _asteapot_game_instance))
  (if (Utilities|Enum|Equal(Enum) _currentstate "NewEnumerator1")
    (Development|PrintString "Spawning Pawn")
    (Networking|SwitchHasAuthority
      (:Authority
        (bind _outactors (Actor|GetAllActorsOfClass "/Script/Engine.PlayerStart"))
        (Variables|Default|SetPlayerStartPoints _outactors)
        (CallFunction|RunonServerSpawnPlayer NewPlayer)))))

(fn ConstructionScript)

(fn NextTurn
  (bind _output_get (Variables|Default|SetTurnIndex (Math|Integer|%(Integer) (+ (Variables|Default|GetTurnIndex) 1) (Utilities|Array|Length (Variables|Default|GetPlayerControllers)))))
  (bind _asteapot_game_state (Utilities|Casting|CastToTeapot_GameState (Game|GetGameState)))
  (bind _output_get_2 (Variables|/Game/Teapot_Content/Blueprints/Teapot_GameState.Teapot_GameState_C|SetTurnIndex _asteapot_game_state _output_get))
  (return _output_get_2))